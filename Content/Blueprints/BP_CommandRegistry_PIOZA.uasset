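; Console command registry for the PIOZA game launcher, where events and functions named after commands parse RawCommand or CommandArgs.
; Most commands drive the W_MainLauncher1 widget found at BeginPlay (repo, games, cache, config) or log diagnostics to the debug console.
; Verify downloads a checksum file, compares MD5s through a ChecksumWorker and re-downloads the game on corruption.
; Shell commands are blocked in distribution builds, and the ShortcutCommand body is unconnected.
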(event `hidetotray`
  (`WindowUtils.MinimizeToTray` "test"))

(event `dcommand`
  (bind _returnvalue (`KismetStringLibrary.ParseIntoArray` (`KismetStringLibrary.Replace` (`self.RawCommand`) "dcommand ")))
  (if (not (`KismetSystemLibrary.IsPackagedForDistribution`))
    (bind (_bsuccess _processid _returnvalue_2) (`ExecCommandLibrary.ExecuteSystemCommand` (`|GetArrayItem` _returnvalue) (`|MakeArray` (`.RightS` (`KismetStringLibrary.Split` (`KismetStringLibrary.JoinStringArray` _returnvalue) " "))) true false 0 "/home/shieldziak/" (`|MakeMap` "")))
    (`/DSHDebugConsole/W_DebugConsole.Send to Log` (`self.DebugConsole`) "NewEnumerator16" _returnvalue_2)))

(event `command`
  (bind _returnvalue (`KismetStringLibrary.Replace` (`self.RawCommand`) "command "))
  (if (not (`KismetSystemLibrary.IsPackagedForDistribution`))
    (bind (_bsuccess _processid _returnvalue_2) (`ExecCommandLibrary.ExecuteSystemCommand` _returnvalue (`KismetStringLibrary.ParseIntoArray` _returnvalue) false false 0 "/home/shieldziak/" (`|MakeMap` "")))
    (`/DSHDebugConsole/W_DebugConsole.Send to Log` (`self.DebugConsole`) "NewEnumerator16" _returnvalue_2)))

(event `setrepo`
  (`RepoCommandLibrary.ExecuteSetRepo` (`self.CommandArgs`) (`/Game/Blueprints/Widgets/W_MainLauncher1.shippingCdnUrl` (`self.MainLauncher`)) (delegate `LogCallback`) (delegate `SetRepoUrlCallback`)))

(event `SetRepoUrlCallback`
  (params (BaseURL :type String) (ManifestName :type String))
  (`/Game/Blueprints/Widgets/W_MainLauncher1.SetRepoURL` (`self.MainLauncher`) BaseURL ManifestName))

(event `LogCallback`
  (params (bIsError :type Boolean) (Message :type String))
  (if bIsError
    (`/DSHDebugConsole/Blueprints/BFL_DebugConsole.LogToConsole` "NewEnumerator12" Message)
    (else
      (`/DSHDebugConsole/Blueprints/BFL_DebugConsole.LogToConsole` "NewEnumerator15" Message))))

(event `self.ReceiveBeginPlay`
  (`parent.ReceiveBeginPlay`)
  (bind _foundwidgets (`WidgetBlueprintLibrary.GetAllWidgetsOfClass` "/Game/Blueprints/Widgets/W_MainLauncher1.W_MainLauncher1_C"))
  (set `self.MainLauncher` (`|GetArrayItem` _foundwidgets)))

(event `verify`
  (`self.VerifyAndRepairGameFiles` (`|GetArrayItem` (`self.CommandArgs`) 1)))

(event `VerifyAndRepairGameFiles`
  (params (GameID :type String))
  (bind (_witharchive _clean _isvalid_) (`/Game/Blueprints/Widgets/W_MainLauncher1.MakeSpecifiedGameURL` (`self.MainLauncher`) GameID))
  (if _isvalid_
    (`FileToStorageDownloader.DownloadFileToStorage` (`KismetStringLibrary.Concat_StrStr` _clean "checksum.txt") (`KismetStringLibrary.Concat_StrStr` (`KismetSystemLibrary.GetProjectSavedDirectory`) "tmp/checksum.txt") 0.0 "text/plain" false (delegate `OnChecksumProgress`) (delegate `OnChecksumDownloaded`))))

(event `OnChecksumProgress`
  (params (BytesReceived :type Integer64) (ContentLength :type Integer64) (ProgressRatio :type "Float (single-precision)")))

(event `OnChecksumDownloaded`
  (params (Result :type "EDownloadToStorageResult Enum" :default "Success") (SavedPath :type String) (Downloader :type "FileToStorageDownloader Object Reference"))
  (switch `EDownloadToStorageResult` Result
    (:`Success`
      (bind (_value _returnvalue) (`BlueprintMapLibrary.Map_Find` (`/Game/Blueprints/Widgets/W_MainLauncher1.GameDirs` (`self.MainLauncher`)) (stale `VerifyAndRepairGameFiles` GameID)))
      (if _returnvalue :!label _label
        (`self.CompareMD5Checksum` SavedPath _value (stale `VerifyAndRepairGameFiles` GameID))))
    (:`SucceededByPayload`
      (goto _label))
    (:`Cancelled`
      (`/DSHDebugConsole/Blueprints/BFL_DebugConsole.LogToConsole` "NewEnumerator12" "Checksum file cannot be downloaded..." :!label _label_2))
    (:`DownloadFailed`
      (goto _label_2))
    (:`SaveFailed`
      (goto _label_2))
    (:`DirectoryCreationFailed`
      (goto _label_2))
    (:`InvalidURL`
      (`/DSHDebugConsole/Blueprints/BFL_DebugConsole.LogToConsole` "NewEnumerator12" "Checksum file not found on server!"))
    (:`InvalidSavePath`
      (goto _label_2))))

(event `compmd5`
  (bind _output (`|GetArrayItem` (`self.CommandArgs`) 1))
  (`self.CompareMD5Checksum` (`|GetArrayItem` (`self.CommandArgs`) 2) (`BlueprintMapLibrary.Map_Find` (`/Game/Blueprints/Widgets/W_MainLauncher1.GameDirs` (`self.MainLauncher`)) _output) _output))

(event `CompareMD5Checksum`
  (params (ChecksumFilePath :type String) (GameDirectoryPath :type String) (GameID :type String))
  (bind _returnvalue (`|GenericCreateObject` "/Game/Blueprints/ChecksumWorker.ChecksumWorker_C"))
  (bind _returnvalue_2 (`BlueprintFileUtilsBPLibrary.FileExists` ChecksumFilePath))
  (if _returnvalue_2
    (`/Game/Blueprints/ChecksumWorker.CompareMD5` :`self` _returnvalue :`ChecksumFilePath` ChecksumFilePath :`GameDirectoryPath` GameDirectoryPath)
    (add `/Game/Blueprints/ChecksumWorker.OnChecksumProgress` _returnvalue (delegate `OnProgress_Event`))
    (add `/Game/Blueprints/ChecksumWorker.OnChecksumComplete` _returnvalue (delegate `OnComplete`))))

(event `OnComplete`
  (params (`AllCorrect?` :type Boolean) (IncorrectFiles :type "Array of String (by ref)"))
  (bind _mainlauncher (`self.MainLauncher`))
  (if `AllCorrect?`
    (`/DSHDebugConsole/Blueprints/BFL_DebugConsole.LogToConsole` "NewEnumerator14" "Verifying complete! All files correct!")
    (`/Game/Blueprints/Libs/PiozaFunctionLIB.BroadcastActionProgress` "NewEnumerator6" 0.0 "Success! No corrupted files found..." "Play!" "NewEnumerator1")
    (else
      (`/DSHDebugConsole/Blueprints/BFL_DebugConsole.LogToConsole` "NewEnumerator12" "FOUND CORRUPTED FILES!")
      (for _array_element IncorrectFiles
        (`/DSHDebugConsole/Blueprints/BFL_DebugConsole.LogToConsole` "NewEnumerator12" _array_element))
      (set `/Game/Blueprints/Widgets/W_MainLauncher1.CurrentGameURL` (`/Game/Blueprints/Widgets/W_MainLauncher1.MakeGameURL` _mainlauncher) _mainlauncher)
      (`KismetSystemLibrary.DelayUntilNextTick`)
      (`/Game/Blueprints/Widgets/W_MainLauncher1.DownloadAndInstall` _mainlauncher))))

(event `OnProgress_Event`
  (params (CurrentFilePath :type String) (FileCount :type Integer) (CurrentFileNumber :type Integer) (`IsCorrect?` :type Boolean) (ProgressPercent :type "Float (double-precision)"))
  (bind _returnvalue (`KismetTextLibrary.Conv_TextToString` (`|FormatText` "{1}/{2} File: {file} | IsCorrect?: {bool}" CurrentFileNumber FileCount CurrentFilePath `IsCorrect?`)))
  (`/Game/Blueprints/Libs/PiozaFunctionLIB.BroadcastActionProgress` "NewEnumerator1" (/ (`KismetMathLibrary.Conv_IntToDouble` CurrentFileNumber) (`KismetMathLibrary.Conv_IntToDouble` FileCount)) "Verifying game files integrity..." "Verifying..." "NewEnumerator2")
  (if `IsCorrect?`
    (`KismetSystemLibrary.PrintString` _returnvalue true false (struct :`R` 1.0 :`B` 0.729591 :`A` 1.0) 10.0 "verif")
    (else
      (`/DSHDebugConsole/Blueprints/BFL_DebugConsole.LogToConsole` "NewEnumerator14" _returnvalue))))

(fn `browse`
  (`/Game/Blueprints/Widgets/W_MainLauncher1.BrowseGame` (`self.MainLauncher`)))

(fn `checkbuilddate`
  (`/DSHDebugConsole/W_DebugConsole.Send to Log` (`self.DebugConsole`) "NewEnumerator15" (`KismetStringLibrary.Concat_StrStr` "BUILD_DATE = " (`BuildDate.GetBuildDate`))))

(fn `checkcache`
  (bind _mainlauncher (`self.MainLauncher`))
  (`/DSHDebugConsole/W_DebugConsole.Send to Log` (`self.DebugConsole`) "NewEnumerator15" (`KismetTextLibrary.Conv_TextToString` (`|FormatText` "Cache statistics:\nHits/Misses\n{hits}/{misses}" (`/Game/Blueprints/Widgets/W_MainLauncher1.CacheHits` _mainlauncher) (`/Game/Blueprints/Widgets/W_MainLauncher1.CacheMisses` _mainlauncher)))))

(fn `checkrhi`
  (`/DSHDebugConsole/W_DebugConsole.Send to Log` (`self.DebugConsole`) "NewEnumerator15" (`KismetStringLibrary.Concat_StrStr` "CURRENT RHI = " (`GetAndSetRHI.GetCurrentRhiName`))))

(fn `clearcache`
  (bind _mainlauncher (`self.MainLauncher`))
  (if (`/Game/Blueprints/Widgets/W_MainLauncher1.IsCacheOnDisk?` _mainlauncher)
    (`/Game/Blueprints/Widgets/W_MainLauncher1.RemoveCache` _mainlauncher)
    (else
      (`/DSHDebugConsole/W_DebugConsole.Send to Log` (`self.DebugConsole`) "NewEnumerator12" "CANNOT DELETE A NON-EXISTENT CACHE!!!"))))

(fn `download`
  (`/Game/Blueprints/Widgets/W_MainLauncher1.InitGameDownload` (`self.MainLauncher`)))

(fn `echo`
  (`/DSHDebugConsole/Blueprints/BFL_DebugConsole.LogToConsole` "NewEnumerator15" (`.RightS` (`KismetStringLibrary.Split` (`self.RawCommand`) "echo "))))

(fn `filedialog`
  (bind _outfilenames (`EFDFunctionLibrary.OpenFileDialog` "" "" "" "" "Single"))
  (for _array_element _outfilenames
    (`/DSHDebugConsole/W_DebugConsole.Send to Log` (`self.DebugConsole`) "NewEnumerator16" _array_element)))

(fn `getcmd`
  (bind _returnvalue (`KismetSystemLibrary.GetCommandLine`))
  (`/DSHDebugConsole/W_DebugConsole.Send to Log` (`self.DebugConsole`) "NewEnumerator14" _returnvalue))

(fn `getlauncherexe`
  (`/DSHDebugConsole/W_DebugConsole.Send to Log` (`self.DebugConsole`) "NewEnumerator15" (`/Game/Blueprints/Libs/PiozaFunctionLIB.GetLauncherExecutable`)))

(fn `getrepo`
  (`/DSHDebugConsole/W_DebugConsole.Send to Log` (`self.DebugConsole`) "NewEnumerator10" (`KismetStringLibrary.Concat_StrStr` "Current repo manifest URL: " (`/Game/Blueprints/Widgets/W_MainLauncher1.CdnUrl` (`self.MainLauncher`)) (`/Game/Blueprints/Saves/LocalConfig.ManifestFileName` (`/Game/Blueprints/Widgets/W_MainLauncher1.Saved Local Config` (`self.MainLauncher`))))))

(fn `list`
  (bind _variable (`|TemporaryVariable`))
  (bind _mainlauncher (`self.MainLauncher`))
  (bind _keys (`BlueprintMapLibrary.Map_Keys` (`.gamesURLs_37_865694942B944B8390906D59FBAF85BA` (break `/Game/Blueprints/Structs/SLauncherManifest` (`/Game/Blueprints/Widgets/W_MainLauncher1.LauncherManifest` _mainlauncher)))))
  (`|AssignmentStatement` _variable)
  (for _array_element _keys
    (bind (_gameid _gameversion _gamebuild _gamechannels _executablenames) (break `/Game/Blueprints/Structs/SGameObjectV2` (`/Game/Blueprints/Libs/PiozaFunctionLIB.GetGameStruct` _array_element)))
    (bind (_value _returnvalue) (`BlueprintMapLibrary.Map_Find` (`/Game/Blueprints/Saves/LocalConfig.SavedGameDirs` (`/Game/Blueprints/Widgets/W_MainLauncher1.Saved Local Config` _mainlauncher)) _gameid))
    (if _returnvalue
      (if (`KismetStringLibrary.IsEmpty` _variable)
        (bind _returnvalue_2 (`KismetStringLibrary.Concat_StrStr` _gameid "  " _value "  " (`BlueprintMapLibrary.Map_Find` _executablenames (`GameplayStatics.GetPlatformName`))))
        (`|AssignmentStatement` _variable _returnvalue_2)
        (else
          (`|AssignmentStatement` _variable (`KismetStringLibrary.Concat_StrStr` _variable " \n" _returnvalue_2))))))
  (`/DSHDebugConsole/W_DebugConsole.Send to Log` (`self.DebugConsole`) "NewEnumerator15" (`KismetTextLibrary.Conv_TextToString` (`|FormatText` "Listing all installed games in following format: \nGameID  InstalledPath  Executable \n{list}" _variable))))

(fn `ls`
  (locals (outputlist :type String) (`all?` :type Boolean))
  (bind _commandargs (`self.CommandArgs`))
  (bind _output (`|GetArrayItem` _commandargs 1))
  (if (`KismetArrayLibrary.Array_Contains` _commandargs "--help")
    (`/DSHDebugConsole/Blueprints/BFL_DebugConsole.LogToConsole` "NewEnumerator15" "Usage: ls [OPTION]... [FILE]...\nList information about the FILEs (the current directory by default).\n  -a, --all                  do not ignore entries starting with .\n      --help                  display this help and exit")
    (elif (`BlueprintPathsLibrary.DirectoryExists` _output)
      (set `local.all?` (or (`KismetArrayLibrary.Array_Contains` _commandargs "-a") (`KismetArrayLibrary.Array_Contains` _commandargs "--all")))
      (if (`BlueprintPathsLibrary.DirectoryExists` _output)
        (bind _outnodes (`FileNodes.ListDirectory` _output "" true true))
        (for _array_element _outnodes
          (if (`KismetStringLibrary.StartsWith` _array_element ".")
            (if (`local.all?`)
              (bind _output_get (set `local.outputlist` (`KismetStringLibrary.Concat_StrStr` (`local.outputlist`) "  " _array_element) :!label _label)))
            (else
              (goto _label))))
        (`/DSHDebugConsole/Blueprints/BFL_DebugConsole.LogToConsole` "NewEnumerator15" _output_get)
        (else
          (`/DSHDebugConsole/Blueprints/BFL_DebugConsole.LogToConsole` "NewEnumerator15" (`KismetTextLibrary.Conv_TextToString` (`|FormatText` "ls: {path}: ls does not have access to this directory!" _output))))))))

(fn `mkmd5`
  (bind _output (`|GetArrayItem` (`self.CommandArgs`) 1))
  (bind (_value _returnvalue) (`BlueprintMapLibrary.Map_Find` (`/Game/Blueprints/Widgets/W_MainLauncher1.GameDirs` (`self.MainLauncher`)) _output))
  (if _returnvalue
    (`/Game/Blueprints/Libs/PiozaFunctionLIB.CalculateMD5` _output (`KismetStringLibrary.Concat_StrStr` _value "/") true)))

(fn `play`
  (bind _mainlauncher (`self.MainLauncher`))
  (bind _mainlauncher_2 (`self.MainLauncher`))
  (bind _output (`|GetArrayItem` (`self.CommandArgs`) 1))
  (if (`.ReturnValue` (`BlueprintMapLibrary.Map_Find` (`/Game/Blueprints/Widgets/W_MainLauncher1.GameStates` _mainlauncher_2) _output))
    (`/Game/Blueprints/Widgets/W_MainLauncher1.SwitchGame` _mainlauncher_2 false (`KismetStringLibrary.Conv_StringToName` _output))
    (switch `/Game/Blueprints/Enums/EGameStatus` (`BlueprintMapLibrary.Map_Find` (`/Game/Blueprints/Widgets/W_MainLauncher1.GameStates` _mainlauncher) (`/Game/Blueprints/Widgets/W_MainLauncher1.CurrentSelectedGameID` _mainlauncher))
      (:`NewEnumerator2`
        (`/Game/Blueprints/Widgets/W_MainLauncher1.LaunchGame` _mainlauncher)))))

(fn `readcache`
  (bind _texturecache (`/Game/Blueprints/Saves/LocalCache.TextureCache` (`/Game/Blueprints/Widgets/W_MainLauncher1.SavedLocalCache` (`self.MainLauncher`))))
  (bind _keys (`BlueprintMapLibrary.Map_Keys` _texturecache))
  (for _array_element _keys
    (`/DSHDebugConsole/W_DebugConsole.Send to Log` (`self.DebugConsole`) "NewEnumerator15" (`KismetStringLibrary.Concat_StrStr` _array_element "\n" (`KismetStringLibrary.Conv_ObjectToString` (`BlueprintMapLibrary.Map_Find` _texturecache _array_element))))))

(fn `reload`
  (params (`Silent?` :type Boolean))
  (if (not `Silent?`)
    (`/DSHDebugConsole/W_DebugConsole.Send to Log` (`self.DebugConsole`) "NewEnumerator11" "DOING A LAUNCHER SOFT-RELOAD ISSUED BY CONSOLE!"))
  (`/Game/Blueprints/Widgets/W_MainLauncher1.ForceLauncherReload` (`self.MainLauncher`) true))

(fn `resetconfig`
  (bind _returnvalue (`BlueprintFileUtilsBPLibrary.DeleteFile` (`KismetStringLibrary.Concat_StrStr` (`KismetSystemLibrary.GetProjectSavedDirectory`) "SaveGames/config.sav")))
  (if _returnvalue
    (`/DSHDebugConsole/W_DebugConsole.Send to Log` (`self.DebugConsole`) "NewEnumerator11" "REMOVED LocalConfig! DOING A LAUNCHER SOFT-RELOAD!")
    (`self.reload` true)
    (else
      (`/DSHDebugConsole/W_DebugConsole.Send to Log` (`self.DebugConsole`) "NewEnumerator12" "FAILED TO REMOVE LocalConfig!"))))

(fn `resetplaytime`
  (bind (_lefts _rights) (`KismetStringLibrary.Split` (`self.RawCommand`) " "))
  (bind _savedplaytime (`/Game/Blueprints/Saves/LocalConfig.SavedPlaytime` (`/Game/Blueprints/Widgets/W_MainLauncher1.Saved Local Config` (`self.MainLauncher`))))
  (if (`.ReturnValue` (`BlueprintMapLibrary.Map_Find` _savedplaytime _rights))
    (`BlueprintMapLibrary.Map_Remove` _savedplaytime _rights)
    (`/DSHDebugConsole/W_DebugConsole.Send to Log` (`self.DebugConsole`) "NewEnumerator15" (`KismetTextLibrary.Conv_TextToString` (`|FormatText` "Playtime for {gamename} was reset!" _rights)))
    (else
      (`/DSHDebugConsole/W_DebugConsole.Send to Log` (`self.DebugConsole`) "NewEnumerator12" (`KismetTextLibrary.Conv_TextToString` (`|FormatText` "Playtime for {gamename} was not found! Check syntax or GameName via command \"list\"" _rights))))))

(fn `rmentry`
  (bind (_lefts _rights) (`KismetStringLibrary.Split` (`self.RawCommand`) "rmentry "))
  (bind _gamedirs (`/Game/Blueprints/Widgets/W_MainLauncher1.GameDirs` (`self.MainLauncher`)))
  (if (`.ReturnValue` (`BlueprintMapLibrary.Map_Find` _gamedirs _rights))
    (bind _returnvalue (`BlueprintMapLibrary.Map_Remove` _gamedirs _rights))
    (if _returnvalue
      (`/DSHDebugConsole/W_DebugConsole.Send to Log` (`self.DebugConsole`) "NewEnumerator15" (`KismetTextLibrary.Conv_TextToString` (`|FormatText` "Removed entry {entry} from list!" _rights)))
      (`/Game/Blueprints/Widgets/W_MainLauncher1.SaveLocalConfig` (`self.MainLauncher`)))
    (else
      (`/DSHDebugConsole/W_DebugConsole.Send to Log` (`self.DebugConsole`) "NewEnumerator12" "Entry with this name does not exist!"))))

(fn `shortcut`
  (bind (_lefts _rights) (`KismetStringLibrary.Split` (`self.RawCommand`) " "))
  (`self.ShortcutCommand` (`KismetStringLibrary.Split` _rights " ") "NewEnumerator0" (`.RightS` (`KismetStringLibrary.Split` _rights " " "IgnoreCase" "FromEnd"))))

(fn `uninstall`
  (if (`Widget.bIsEnabled` (`/Game/Blueprints/Widgets/W_MainLauncher1.UninstallB` (`self.MainLauncher`)))
    (`/Game/Blueprints/Widgets/W_MainLauncher1.UninstallGame` (`self.MainLauncher`) "")
    (else
      (`/DSHDebugConsole/W_DebugConsole.Send to Log` (`self.DebugConsole`) "NewEnumerator12" "YOU CANNOT UNINSTALL A NON-EXISTENT GAME!!!"))))

(fn `updaterepo`
  (`/Game/Blueprints/Widgets/W_MainLauncher1.Trigger Force Update Repo` (`self.MainLauncher`)))

(fn `UserConstructionScript`
  (`parent.UserConstructionScript`))

(fn `volume`
  (bind _rawcommand (`self.RawCommand`))
  (bind _returnvalue (`KismetStringLibrary.Conv_StringToDouble` (`KismetStringLibrary.Replace` _rawcommand "volume ")))
  (if (`KismetStringLibrary.Contains` _rawcommand "default")
    (`GameplayStatics.SetSoundMixClassOverride` "/Game/Media/SFX_MIX.SFX_MIX" "/Game/Media/SC_SFX.SC_SFX" 1.0 1.0 0.0)
    (`/DSHDebugConsole/W_DebugConsole.Send to Log` (`self.DebugConsole`) "NewEnumerator14" (`KismetStringLibrary.Concat_StrStr` "CHANGED AUDIO VOLUME TO: " "1.0"))
    (else
      (`GameplayStatics.SetSoundMixClassOverride` "/Game/Media/SFX_MIX.SFX_MIX" "/Game/Media/SC_SFX.SC_SFX" _returnvalue 1.0 0.0)
      (`/DSHDebugConsole/W_DebugConsole.Send to Log` (`self.DebugConsole`) "NewEnumerator14" (`KismetStringLibrary.Concat_StrStr` "CHANGED AUDIO VOLUME TO: " (`KismetStringLibrary.Conv_DoubleToString` _returnvalue))))))