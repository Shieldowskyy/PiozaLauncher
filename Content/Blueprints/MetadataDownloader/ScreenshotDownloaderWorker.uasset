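; Worker that downloads one numbered game screenshot for the launcher's metadata downloader into the project's Saved meta folder.
; It compares the remote content size with the cached file and skips matches, reporting them as unsuccessful with an empty path.
; Otherwise it downloads to memory, saves after a loose OR-chained content check, and reports through CallOnFinished.
; A failed attempt gets one timer-delayed retry; texture caching is disconnected, noted as crashing VRAM.
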(event `DownloadScreenshot`
  (params (MetaGameURL :type String) (MetaGameName :type String) (ScreenshotNumber :type Integer))
  (bind _meta_game_name (`self.Meta Game Name`))
  (bind _screenfilename (`self.ScreenFileName`))
  (bind _verbose_ (`self.Verbose?`))
  (set `self.MetaGameURL` MetaGameURL)
  (set `self.Meta Game Name` MetaGameName)
  (set `self.ScreenshotNumber` ScreenshotNumber)
  (bind _output_get (set `self.ScreenFileName` (`KismetStringLibrary.Concat_StrStr` "screen" (`KismetStringLibrary.Conv_IntToString` (`self.ScreenshotNumber`)) ".jpg")))
  (bind _output_get_2 (set `self.ScreenURL` (`KismetStringLibrary.Concat_StrStr` (`self.MetaGameURL`) "meta/screens/" _output_get)))
  (set `self.ScreenSavePath` (`KismetStringLibrary.Concat_StrStr` (`KismetSystemLibrary.GetProjectSavedDirectory`) "meta/" _meta_game_name "/screens/" _screenfilename))
  (`KismetSystemLibrary.PrintText` null (`|FormatText` "[SCREENSHOT-WORKER]\nStarting downloading screenshot:\n{GameName}\n{path}" _meta_game_name _screenfilename) _verbose_ _verbose_ (struct :`R` 1.0 :`B` 0.849339 :`A` 1.0) 20.0)
  (`BaseFilesDownloader.GetContentSize` _output_get_2 1.0 (delegate `ScreenshotContentSize`)))

(event `OnScreenshotDownloaded`
  (params (DownloadedContent :type "Array of Byte (by ref)") (Result :type "EDownloadToMemoryResult Enum" :default "Success") (Downloader :type "FileToMemoryDownloader Object Reference"))
  (bind _verbose_ (`self.Verbose?`))
  (bind _screensavepath (`self.ScreenSavePath`))
  (bind _verbose__2 (`self.Verbose?`))
  (bind _verbose__3 (`self.Verbose?`))
  (bind _verbose__4 (`self.Verbose?`))
  (bind _returnvalue (`BaseFilesDownloader.BytesToString` DownloadedContent))
  (if (and (`|EnumEquality` Result "Success") (or (`KismetStringLibrary.Contains` _returnvalue "PNG") (not (`KismetStringLibrary.Contains` _returnvalue "DOCTYPE")) (not (`KismetStringLibrary.Contains` _returnvalue "<?xml"))))
    (`KismetSystemLibrary.PrintString` (`self.MainLauncher`) "SAVING PNG FILE..." _verbose_ _verbose_ (struct :`R` 0.289773 :`G` 1.0 :`A` 1.0) 5.0)
    (`BaseFilesDownloader.SaveArrayToFile` DownloadedContent _screensavepath)
    (`self.OnFinished` true (`self.ScreenshotNumber`) _screensavepath)
    (`KismetSystemLibrary.PrintText` null (`|FormatText` "[SCREENSHOT-WORKER]\nSUCCESS downloading screenshot:\n{GameName}\n{path}" (`self.Meta Game Name`) (`self.ScreenFileName`)) _verbose__3 _verbose__3 (struct :`R` 0.324311 :`G` 1.0 :`A` 1.0) 20.0)
    (else
      (`KismetSystemLibrary.PrintString` (`self.MainLauncher`) "NOT A PNG FILE! CANCELLING SAVING PROCESS AND SKIPPING..." _verbose__4 _verbose__4 (struct :`R` 1.0 :`G` 0.104234 :`A` 1.0) 6.0)
      (if (`self.Retried?`)
        (`self.OnFinished` false (`self.ScreenshotNumber`) _screensavepath)
        (`KismetSystemLibrary.PrintText` null (`|FormatText` "[SCREENSHOT-WORKER]\nERROR downloading screenshot:\n{GameName}\n{path}\nResponse: {response}" (`self.Meta Game Name`) (`self.ScreenFileName`) _returnvalue) _verbose__2 _verbose__2 (struct :`R` 1.0 :`G` 0.022284 :`A` 1.0) 20.0)
        (else
          (`KismetSystemLibrary.K2_SetTimerDelegate` (`|CreateDelegate` :!event `RetryScreenshotDownload`) 0.25 false true))))))

(event `OnScreensotDownloadProgress`
  (params (BytesReceived :type Integer64) (ContentLength :type Integer64) (ProgressRatio :type "Float (single-precision)")))

(event `ScreenshotContentSize`
  (params (ContentLength :type Integer64))
  (bind _verbose_ (`self.Verbose?`))
  (bind _verbose__2 (`self.Verbose?`))
  (bind _returnvalue (`FileNodes.GetFileSize` (`self.ScreenSavePath`)))
  (if (== _returnvalue ContentLength)
    (`KismetSystemLibrary.PrintString` (`self.MainLauncher`) "SCREENSHOT IDENTICAL TO CACHED! SKIPPING..." _verbose_ _verbose_ (struct :`R` 1.0 :`G` 0.104234 :`A` 1.0) 6.0)
    (`self.OnFinished` false (`self.ScreenshotNumber`))
    (`KismetSystemLibrary.PrintText` null (`|FormatText` "[SCREENSHOT-WORKER]\nCACHED downloading screenshot:\n{GameName}\n{path}" (`self.Meta Game Name`) (`self.ScreenFileName`)) _verbose__2 _verbose__2 (struct :`R` 1.0 :`G` 0.672844 :`A` 1.0) 20.0)
    (else
      (`FileToMemoryDownloader.DownloadFileToMemory` (`self.ScreenURL`) 0.0 "image/x-jpg" false (delegate `OnScreensotDownloadProgress`) (delegate `OnScreenshotDownloaded`) :!label _label))))

(event `RetryScreenshotDownload`
  (set `self.Retried?` true)
  (goto _label))