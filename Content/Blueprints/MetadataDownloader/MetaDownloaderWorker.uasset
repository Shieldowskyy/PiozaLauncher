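; Worker Blueprint that downloads one metadata file for a named game into the project's Saved meta folder and reports when finished.
; DownloadMeta builds the URL and save path, then checks remote content size, skipping files that match the cached size or fall under a small minimum.
; Successful JPG downloads schedule a short timer, apparently for a single repeat download via the Retried flag.
; Failures are logged and still signal completion.
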(event `DownloadMeta`
  (params (CurrentMetaFileName :type String) (CurrentMetaGameName :type String) (CurrentMetaGameURL :type String))
  (set `self.Current Meta File Name` CurrentMetaFileName)
  (set `self.Current Meta Game Name` CurrentMetaGameName)
  (set `self.Current Meta Game URL` CurrentMetaGameURL)
  (set `self.MetaSavePath` (`KismetStringLibrary.Concat_StrStr` (`KismetSystemLibrary.GetProjectSavedDirectory`) "meta/" (`self.Current Meta Game Name`) "/" (`self.Current Meta File Name`)))
  (bind _output_get (set `self.MetaDownloadURL` (`KismetStringLibrary.Concat_StrStr` (`self.Current Meta Game URL`) "meta/" (`self.Current Meta File Name`))))
  (`BaseFilesDownloader.GetContentSize` _output_get 1.0 (delegate `CheckedContentSize`)))

(event `OnFileDownloadCompleted`
  (params (Result :type "EDownloadToStorageResult Enum" :default "Success") (SavedPath :type String) (Downloader :type "FileToStorageDownloader Object Reference"))
  (bind _verbose_ (`self.Verbose?`))
  (bind _verbose__2 (`self.Verbose?`))
  (if (or (`|EnumEquality` Result "Success") (`|EnumEquality` Result "SucceededByPayload"))
    (`KismetSystemLibrary.PrintString` null (`KismetStringLibrary.Concat_StrStr` "Save file path: " SavedPath) _verbose_ _verbose_)
    (if (`KismetStringLibrary.EndsWith` (`self.Current Meta File Name`) ".jpg")
      (if (`self.Retried?`)
        (`self.OnFinished` (`self.Current Meta File Name`))
        (else
          (`KismetSystemLibrary.K2_SetTimerDelegate` (`|CreateDelegate` :!event `RetryFileDownload`) 0.25 false true)))
      (else
        (`self.OnFinished` (`self.Current Meta File Name`) :!label _label)))
    (else
      (`KismetSystemLibrary.PrintText` null (`|FormatText` "FAILED TO DOWNLOAD META FILE!\nPath : {path}\nError: {err}" (`self.MetaSavePath`) (`|GetEnumeratorNameAsString` Result)) _verbose__2 _verbose__2 (struct :`R` 1.0 :`G` 0.009755 :`A` 1.0) 12.0)
      (goto _label))))

(event `CheckedContentSize`
  (params (ContentLength :type Integer64))
  (bind _verbose_ (`self.Verbose?`))
  (bind _verbose__2 (`self.Verbose?`))
  (bind _returnvalue (`FileNodes.GetFileSize` (`self.MetaSavePath`)))
  (if (or (== ContentLength _returnvalue) (< ContentLength 2048))
    (`KismetSystemLibrary.PrintString` null "ASSET IDENTICAL TO CACHED OR TOO SMALL! SKIPPING..." _verbose_ _verbose_ (struct :`R` 1.0 :`G` 0.104234 :`A` 1.0) 6.0)
    (`self.OnFinished` (`self.Current Meta File Name`))
    (else
      (`FileToStorageDownloader.DownloadFileToStorage` (`self.MetaDownloadURL`) (`self.MetaSavePath`) 0.0 "application/octet-stream" false (delegate `OnFileDownloading`) (`|CreateDelegate` :!event `OnFileDownloadCompleted`) :!label _label_2)
      (`KismetSystemLibrary.PrintText` null (`|FormatText` "Downloading {filename} for {GameName}..." (`self.Current Meta File Name`) (`self.Current Meta Game Name`)) _verbose__2 _verbose__2 (struct :`R` 1.0 :`G` 0.964345 :`A` 1.0) 6.0))))

(event `OnFileDownloading`
  (params (BytesReceived :type Integer64) (ContentLength :type Integer64) (ProgressRatio :type "Float (single-precision)")))

(event `RetryFileDownload`
  (set `self.Retried?` true)
  (goto _label_2))