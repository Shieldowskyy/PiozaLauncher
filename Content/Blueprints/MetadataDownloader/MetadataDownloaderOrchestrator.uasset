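; Launcher actor that downloads metadata files and screenshots for every game in the manifest, shows progress on MainLauncher, then destroys itself.
; Games run sequentially: each gets a saved folder and one parallel MetaDownloaderWorker per file.
; Once those drain via next-tick polling, ScreenshotDownloaderWorkers fetch numbered screenshots, capped at MaxConcurrent.
; The first failed screenshot stops queuing, and NextGame advances the loop when active workers finish.
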(event `DownloadNextFile`
  (if (< (`self.ActiveWorkers`) (`self.MaxConcurrent`)) :!label _label
    (`self.ShowDownloadingMediaText` "media")
    (else
      (`KismetSystemLibrary.DelayUntilNextTick`)
      (goto _label))))

(event `NextGame`
  (bind _filesdownloading (`self.FilesDownloading`))
  (goto _label_3 :!via `Next`))

(event `OnScreenshotDownloaded`
  (params (`Success?` :type Boolean) (ScreenNum :type Integer) (FilePath :type String))
  (`/Engine/EditorBlueprintResources/StandardMacros.DecrementInt` (`self.ActiveWorkers`)
    (:`  `
      (if `Success?`
        (`KismetSystemLibrary.Delay` 0.1)
        (`self.QueueScreenshotWorker`)
        (else
          (set `self.AbortProcessing?` true)
          (if (< (`self.ActiveWorkers`) 1) :!label _label_2
            (`self.NextGame`)
            (set `self.ScreenshotNumber` -1)
            (else
              (`KismetSystemLibrary.DelayUntilNextTick`)
              (goto _label_2))))))))

(event `QueueScreenshotWorker`
  (if (`self.AbortProcessing?`)
    _
    (elif (< (`self.ActiveWorkers`) (`self.MaxConcurrent`))
      (`/Engine/EditorBlueprintResources/StandardMacros.IncrementInt` (`self.ScreenshotNumber`)
        (:`  `
          (`/Engine/EditorBlueprintResources/StandardMacros.IncrementInt` (`self.ActiveWorkers`)
            (:`  `
              (bind _returnvalue (`|GenericCreateObject` "/Game/Blueprints/MetadataDownloader/ScreenshotDownloaderWorker.ScreenshotDownloaderWorker_C" (`self.MainLauncher`)))
              (add `/Game/Blueprints/MetadataDownloader/ScreenshotDownloaderWorker.OnFinished` _returnvalue (delegate `OnScreenshotDownloaded`))
              (`/Game/Blueprints/MetadataDownloader/ScreenshotDownloaderWorker.DownloadScreenshot` _returnvalue (`self.CurrentMetaGameURL`) (`self.CurrentMetaGameName`) (`self.ScreenshotNumber`))
              (`KismetSystemLibrary.Delay` 0.1)
              (`self.QueueScreenshotWorker`))))))))

(event `DownloadScreenshots`
  (bind _verbose_ (`self.Verbose?`))
  (set `self.ActiveWorkers` 0)
  (set `self.AbortProcessing?` false)
  (set `self.ScreenshotNumber` -1)
  (`self.ShowDownloadingMediaText` "screenshots")
  (`KismetSystemLibrary.PrintText` (`|FormatText` "[SCREENSHOT-WORKER]\nStarting screenshot downloading for game {gamename}!\nThreadLimit: {Limit}" (`self.CurrentMetaGameName`) (`self.MaxConcurrent`)) _verbose_ _verbose_ (struct :`R` 1.0 :`B` 0.849339 :`A` 1.0) 20.0)
  (`self.QueueScreenshotWorker`))

(event `QueueMetaWorker`
  (params (CurrentMetaFileName :type String))
  (bind _verbose_ (`self.Verbose?`))
  (bind _currentmetagameurl (`self.CurrentMetaGameURL`))
  (bind _currentmetagamename (`self.CurrentMetaGameName`))
  (`/Engine/EditorBlueprintResources/StandardMacros.IncrementInt` (`self.ActiveWorkers`)
    (:`  `
      (bind _returnvalue (`|GenericCreateObject` "/Game/Blueprints/MetadataDownloader/MetaDownloaderWorker.MetaDownloaderWorker_C" (`self.MainLauncher`)))
      (add `/Game/Blueprints/MetadataDownloader/MetaDownloaderWorker.OnFinished` _returnvalue (delegate `OnMetaFileDownloaded`))
      (`/Game/Blueprints/MetadataDownloader/MetaDownloaderWorker.DownloadMeta` _returnvalue CurrentMetaFileName _currentmetagamename _currentmetagameurl)
      (`KismetSystemLibrary.PrintText` (`|FormatText` "Constructed MetaWorker with task:\nFileName: {FileName}\nGameName: {GameName}\nURL: {URL}" CurrentMetaFileName _currentmetagamename _currentmetagameurl) _verbose_ _verbose_ (struct :`R` 0.844622 :`B` 1.0 :`A` 1.0) 8.0))))

(event `OnMetaFileDownloaded`
  (params (FileName :type String))
  (`KismetArrayLibrary.Array_RemoveItem` (`self.FilesDownloading`) FileName)
  (`/Engine/EditorBlueprintResources/StandardMacros.DecrementInt` (`self.ActiveWorkers`)))

(event `self.ReceiveBeginPlay`
  (bind _filesdownloading (`self.FilesDownloading`))
  (bind ((`minSupportedVersion_43_AF634A1AD4E542208FB2C8470CDB138D` _minsupportedversion) (`latestVersion_45_FB94109C99F44AC28986A983DDE07EDF` _latestversion) (`gamesURLs_37_865694942B944B8390906D59FBAF85BA` _gamesurls)) (break `/Game/Blueprints/Structs/SLauncherManifest` (`self.SLauncher Manifest`)))
  (bind _keys (`BlueprintMapLibrary.Map_Keys` _gamesurls))
  (bind (_array_element _array_index) (`/Game/Blueprints/Libs/PiozaMacroLIB.ForEachLoopWithDelay` _keys :!label _label_3)
    (:`LoopBody`
      (set `self.CurrentMetaGameName` _array_element)
      (set `self.CurrentMetaGameURL` (`BlueprintMapLibrary.Map_Find` _gamesurls (`self.CurrentMetaGameName`)))
      (bind _returnvalue (`KismetArrayLibrary.Array_Length` _keys))
      (set `TextBlock.Text` (`|FormatText` "Refreshing metadata ({current}/{length})" (+ _array_index 1) _returnvalue) (`/Game/Blueprints/Widgets/W_MainLauncher1.MetadataText` (`self.MainLauncher`)))
      (`ProgressBar.SetPercent` (`/Game/Blueprints/Widgets/W_MainLauncher1.RefreshingProgress` (`self.MainLauncher`)) (/ (/ 100 (- _returnvalue _array_index)) 100.0))
      (bind _returnvalue_2 (`BlueprintFileUtilsBPLibrary.MakeDirectory` (`KismetStringLibrary.Concat_StrStr` (`KismetSystemLibrary.GetProjectSavedDirectory`) "meta/" (`self.CurrentMetaGameName`)) true))
      (if _returnvalue_2
        (`self.ShowDownloadingMediaText` "media")
        (`KismetArrayLibrary.Array_Clear` (`self.FilesDownloading`))
        (for _array_element_2 (`self.MetaFileNames`)
          (if (not (`KismetArrayLibrary.Array_Contains` _filesdownloading _array_element_2))
            (`KismetArrayLibrary.Array_Add` _filesdownloading _array_element_2)
            (`self.QueueMetaWorker` _array_element_2)))
        (if (< (`self.ActiveWorkers`) 1) :!label _label_4
          (`self.DownloadScreenshots`)
          (else
            (`KismetSystemLibrary.DelayUntilNextTick`)
            (goto _label_4)))
        (else
          (`/Game/Blueprints/Widgets/W_MainLauncher1.CustomError` (`self.MainLauncher`) "Failed to create folder tree for games metadata files!\nCheck free disk space or permissions or try reinstalling or updating launcher..."))))
    (:`Completed`
      (`self.OnMetadataDownloadCompleted`)
      (`self.K2_DestroyActor`))))

(fn `ShowDownloadingMediaText`
  (params (ContentType :type Text))
  (set `TextBlock.Text` (`|FormatText` "Downloading {type} for {GameName}..." ContentType (`self.CurrentMetaGameName`)) (`/Game/Blueprints/Widgets/W_MainLauncher1.MetadataDesc` (`self.MainLauncher`))))

(fn `UserConstructionScript`)