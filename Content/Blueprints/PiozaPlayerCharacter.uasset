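; PiozaPlayerCharacter is the player character that hosts the game launcher UI and routes keyboard and action input to it.
; On BeginPlay it creates the W_MainLauncher1 widget and sets Game and UI input, while Tick keeps the mouse cursor visible.
; Input events call the widget to toggle the console, switch or add games, open menus, or reload the launcher in non-distribution builds.
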(event `self.ReceiveBeginPlay`
  (bind _returnvalue (`GameplayStatics.GetPlayerController` 0))
  (bind _returnvalue_2 (`|CreateWidget` "/Game/Blueprints/Widgets/W_MainLauncher1.W_MainLauncher1_C" _returnvalue))
  (set `self.MainLauncherW` _returnvalue_2)
  (`UserWidget.AddToViewport` _returnvalue_2 0)
  (`WidgetBlueprintLibrary.SetInputMode_GameAndUIEx` _returnvalue null "DoNotLock" false true))

(event `self.ReceiveTick`
  (params (DeltaSeconds :type "Float (single-precision)"))
  (set `PlayerController.bShowMouseCursor` true (`GameplayStatics.GetPlayerController` 0)))

(event `Key|Tilde`
  (params (Key :type "Key Structure"))
  (:`Pressed`
    (`/Game/Blueprints/Widgets/W_MainLauncher1.ToggleConsole` (`self.MainLauncherW`))))

(event `InputAction|ReloadLauncher`
  (params (Key :type "Key Structure"))
  (:`Pressed`
    (if (not (`KismetSystemLibrary.IsPackagedForDistribution`))
      (`/Game/Blueprints/Widgets/W_MainLauncher1.ForceLauncherReload` (`self.MainLauncherW`) false))))

(event `InputAction|NextGame`
  (params (Key :type "Key Structure"))
  (:`Pressed`
    (`/Game/Blueprints/Widgets/W_MainLauncher1.SwitchToNextGame` (`self.MainLauncherW`))))

(event `InputAction|PreviousGame`
  (params (Key :type "Key Structure"))
  (:`Pressed`
    (`/Game/Blueprints/Widgets/W_MainLauncher1.SwitchToPreviousGame` (`self.MainLauncherW`))))

(event `InputAction|AddCustomGame`
  (params (Key :type "Key Structure"))
  (bind _mainlauncherw (`self.MainLauncherW`))
  (:`Pressed`
    (if (`Widget.bIsEnabled` (`/Game/Blueprints/Widgets/W_MainLauncher1.AddGameButton` _mainlauncherw))
      (`/Game/Blueprints/Widgets/W_MainLauncher1.ShowAddGameWizard` _mainlauncherw))))

(event `InputAction|OpenOptionsMenu`
  (params (Key :type "Key Structure"))
  (:`Pressed`
    (`/Game/Blueprints/Widgets/W_MainLauncher1.OpenOptionsMenu` (`self.MainLauncherW`))))

(event `Key|F1`
  (params (Key :type "Key Structure"))
  (:`Pressed`
    (`/Game/Blueprints/Widgets/W_MainLauncher1.OpenAboutMenu` (`self.MainLauncherW`))))

(fn `UserConstructionScript`)