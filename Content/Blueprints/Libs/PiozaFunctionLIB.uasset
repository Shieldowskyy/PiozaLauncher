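; Blueprint function library of shared helpers for the Pioza game launcher on Windows and Linux.
; File helpers resolve per-game meta and umu paths, parse game.json into SGameObjectV2, and compute MD5 manifests.
; UI helpers recursively theme borders and buttons, pick localized strings with English fallback, and broadcast progress through BPI_Pioza.
; Free-space checks query the drive root on Windows; on Linux they create a missing directory first, a workaround flagged unsafe.
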(fn `AddChildWidgetAtIndex`
  (params (ScrollBox :type "PanelWidget Object Reference") (ChildWidget :type "Widget Object Reference (by ref)") (Index :type Integer))
  (returns (AddedChild :type "PanelSlot Object Reference"))
  (locals (L_WidgetsArray :type "Array of Widget Object Reference"))
  (bind _output_get (set `local.L_WidgetsArray` (`PanelWidget.GetAllChildren` ScrollBox)))
  (`KismetArrayLibrary.Array_Insert` _output_get ChildWidget Index)
  (`PanelWidget.ClearChildren` ScrollBox)
  (for _array_element (`local.L_WidgetsArray`)
    (bind _returnvalue (`PanelWidget.AddChild` ScrollBox _array_element)))
  (return _returnvalue))

(fn `BroadcastActionProgress`
  (params (BusyState :type "/Game/Blueprints/Enums/EBusyState Enum" :default "NewEnumerator12") (Progress :type "Float (double-precision)") (Message :type Text) (ActionButtonText :type Text) (ActionButtonStatus :type "/Game/Blueprints/Enums/EButtonEnabled Enum" :default "NewEnumerator0"))
  (bind _foundwidgets (`WidgetBlueprintLibrary.GetAllWidgetsWithInterface` null "/Game/Blueprints/Interfaces/BPI_Pioza.BPI_Pioza_C"))
  (message `/Game/Blueprints/Interfaces/BPI_Pioza.BroadcastActionProgress` _foundwidgets BusyState Progress Message ActionButtonText ActionButtonStatus))

(fn `BytesToMB`
  (params (A :type Integer64))
  (returns (ReturnValue :type Integer64))
  (return (/ (/ A 1024) 1000)))

(fn `CalculateMD5`
  (params (GameID :type String) (GamePath :type String) (`SaveToFile?` :type Boolean))
  (returns (FileChecksums :type "Map of String to String"))
  (locals (LocalResult :type String) (LocalGameID :type String) (LocalGamePath :type String) (LocalFileChecksums :type "Map of String to String"))
  (bind _returnvalue (`KismetStringLibrary.Concat_StrStr` (`KismetStringLibrary.Concat_StrStr` (`KismetSystemLibrary.GetProjectSavedDirectory`) "md5/" GameID "/") "checksum-" (`GameplayStatics.GetPlatformName`) ".txt"))
  (set `local.LocalGameID` GameID)
  (bind _returnvalue_2 (`BlueprintFileUtilsBPLibrary.DirectoryExists` GamePath))
  (if _returnvalue_2
    (set `local.LocalGamePath` GamePath)
    (bind (_outnodes _returnvalue_3) (`FileNodes.ListDirectory` (`local.LocalGamePath`) "" true false true))
    (if _returnvalue_3
      (for _array_element _outnodes
        (bind (_outchecksum _returnvalue_4) (`ChecksumLibrary.CalculateFileChecksum` _array_element "MD5"))
        (if _returnvalue_4
          (bind _output_get (set `local.LocalResult` (`KismetStringLibrary.Concat_StrStr` (`local.LocalResult`) "\n" (`KismetTextLibrary.Conv_TextToString` (`|FormatText` "{checksum} {file}" _outchecksum (`KismetStringLibrary.Replace` _array_element (`local.LocalGamePath`)))))))
          (`BlueprintMapLibrary.Map_Add` (`local.LocalFileChecksums`) _array_element _outchecksum)))
      (if `SaveToFile?`
        (bind (_outerror _returnvalue_5) (`FileNodes.SaveText` _returnvalue _output_get false false "UTF8WithoutBOM"))
        (if _returnvalue_5
          (`/DSHDebugConsole/Blueprints/BFL_DebugConsole.LogToConsole` "NewEnumerator14" (`KismetStringLibrary.Concat_StrStr` "SUCCESSFULLY CALCULATED MD5! RESULT FILE PATH: " _returnvalue))
          (return (`local.LocalFileChecksums`)))
        (else
          (`/DSHDebugConsole/Blueprints/BFL_DebugConsole.LogToConsole` "NewEnumerator14" "SUCCESSFULLY CALCULATED MD5!")
          (return (`local.LocalFileChecksums`)))))
    (else
      (`/DSHDebugConsole/Blueprints/BFL_DebugConsole.LogToConsole` "NewEnumerator12" "DESIRED GAME NOT INSTALLED!!!"))))

(fn `CleanFilename`
  (params (SourceString :type String))
  (returns (ReturnValue :type String))
  (locals (ModifiedString :type String))
  (set `local.ModifiedString` SourceString)
  (for _array_element (`KismetStringLibrary.GetCharacterArrayFromString` ":/\\?<>*\"|'")
    (set `local.ModifiedString` (`KismetStringLibrary.Replace` (`local.ModifiedString`) _array_element)))
  (return (`local.ModifiedString`)))

(fn `CleanJsonString`
  (params (SourceString :type String))
  (returns (ReturnValue :type String))
  (locals (ModifiedString :type String))
  (set `local.ModifiedString` SourceString)
  (for _array_element (`KismetStringLibrary.GetCharacterArrayFromString` "\"\\")
    (set `local.ModifiedString` (`KismetStringLibrary.Replace` (`local.ModifiedString`) _array_element)))
  (return (`local.ModifiedString`)))

(fn `ConvertCmdLineToArray`
  (params (RawCommandString :type String))
  (returns (ParsedArgs :type "Array of String"))
  (locals (TempList :type "Array of String"))
  (bind (_outtokens _outswitches _outparams) (`KismetSystemLibrary.ParseCommandLine` RawCommandString))
  ; Switches
  (for _array_element _outswitches
    (`KismetArrayLibrary.Array_Add` (`local.TempList`) (`KismetStringLibrary.Concat_StrStr` "-" _array_element)))
  ; Params
  (bind _keys (`BlueprintMapLibrary.Map_Keys` _outparams))
  (for _array_element_2 _keys
    (`KismetArrayLibrary.Array_Add` (`local.TempList`) (`KismetStringLibrary.Concat_StrStr` "-" _array_element_2 "=" (`BlueprintMapLibrary.Map_Find` _outparams _array_element_2))))
  (`KismetArrayLibrary.Array_Append` (`local.TempList`) _outtokens)
  (return (`local.TempList`)))

(fn `FindLocalizableString`
  (params (TargetMap :type "Map of String to String (by ref)"))
  (returns (ReturnValue :type String) (`found?` :type Boolean))
  (locals (FoundVar :type String) (Success :type Boolean))
  (bind (_value _returnvalue) (`BlueprintMapLibrary.Map_Find` TargetMap "en"))
  (bind (_value_2 _returnvalue_2) (`BlueprintMapLibrary.Map_Find` TargetMap (`KismetInternationalizationLibrary.GetCurrentLanguage`)))
  (if _returnvalue_2
    (bind _output_get (set `local.FoundVar` _value_2))
    (bind _output_get_2 (set `local.Success` true))
    (return _output_get _output_get_2)
    (elif _returnvalue
      (bind _output_get_3 (set `local.FoundVar` _value))
      (bind _output_get_4 (set `local.Success` true))
      (return _output_get_3 _output_get_4)
      (else
        (bind _output_get_5 (set `local.Success` false))
        (return "" _output_get_5)))))

(fn `GetGameStruct`
  (params (RowName :type String))
  (returns (ReturnValue :type "/Game/Blueprints/Structs/SGameObjectV2 Structure") (`IsValid?` :type Boolean))
  (locals (`Valid?` :type Boolean :default false))
  (bind (_outtext _returnvalue) (`FileNodes.ReadText` (`KismetStringLibrary.Concat_StrStr` (`KismetSystemLibrary.GetProjectSavedDirectory`) "meta/" RowName "/game.json")))
  (if _returnvalue
    (bind _outstruct (`JsonParserLib.JsonToStruct` _outtext "/Game/Blueprints/Structs/SGameObjectV2.SGameObjectV2"))
    (bind _value (`BlueprintInstancedStructLibrary.GetInstancedStructValue` _outstruct)
      (:`Valid`
        (set `local.Valid?` true))))
  (return _value (`local.Valid?`)))

(fn `GetLauncherConfig`
  (returns (ConfigStruct :type "/Game/Blueprints/Structs/SLauncherConfig Structure"))
  (locals (LauncherConfig :type "/Game/Blueprints/PrimaryDataAssets/PDA_LauncherConfig Object Reference" :default "/Game/Blueprints/PrimaryDataAssets/PDA_LauncherConfig.PDA_LauncherConfig_C'/Game/Data/LauncherConfig.LauncherConfig'"))
  (return (`/Game/Blueprints/PrimaryDataAssets/PDA_LauncherConfig.Config` (`local.LauncherConfig`))))

(fn `GetLauncherExecutable`
  (returns (ReturnValue :type String))
  (locals (Final :type String))
  (switch `string` (`GameplayStatics.GetPlatformName`)
    (:`Windows`
      (set `local.Final` (`KismetStringLibrary.Concat_StrStr` (`KismetSystemLibrary.GetProjectDirectory`) (`KismetSystemLibrary.GetGameName`) ".exe")))
    (:`Linux`
      (bind _output_get (set `local.Final` (`KismetStringLibrary.Concat_StrStr` (`KismetSystemLibrary.GetProjectDirectory`) (`KismetSystemLibrary.GetGameName`))))))
  (return _output_get))

(fn `GetMetaFilePath`
  (params (GameID :type String) (FileWithExtension :type String))
  (returns (FilePath :type String) (ReturnValue :type Boolean))
  (bind _returnvalue (`KismetSystemLibrary.ConvertToAbsolutePath` (`KismetStringLibrary.Concat_StrStr` (`KismetSystemLibrary.GetProjectSavedDirectory`) "meta/" GameID "/" FileWithExtension)))
  (return _returnvalue (`BlueprintPathsLibrary.FileExists` _returnvalue)))

(fn `GetPlatformFreeDiskSpaceInMB`
  (params (`Directory Path` :type String))
  (returns (`Return Value` :type Integer64))
  (locals (LocalFinal :type Integer64 :default 0) (LocalPath :type String))
  (bind _returnvalue (`KismetStringLibrary.GetCharacterArrayFromString` (`local.LocalPath`)))
  (set `local.LocalPath` `Directory Path`)
  (switch `string` (`GameplayStatics.GetPlatformName`)
    (:`Windows`
      (bind _returnvalue_2 (`CheckDiskSpace.GetFreeDiskSpaceInMB` (`KismetStringLibrary.Concat_StrStr` (`|GetArrayItem` _returnvalue) (`|GetArrayItem` _returnvalue 1) (`|GetArrayItem` _returnvalue 2))))
      (bind _output_get (set `local.LocalFinal` _returnvalue_2)))
    (:`Linux`
      (bind _returnvalue_3 (`BlueprintFileUtilsBPLibrary.DirectoryExists` (`local.LocalPath`)))
      (if _returnvalue_3
        (bind _returnvalue_4 (`CheckDiskSpace.GetFreeDiskSpaceInMB` (`local.LocalPath`) :!label _label))
        (set `local.LocalFinal` _returnvalue_4)
        (else
          (bind _returnvalue_5 (`BlueprintFileUtilsBPLibrary.MakeDirectory` (`local.LocalPath`))) ; WARNING! FUCKING UNSAFE WORKAROUND. MAY INTERFERE WITH USER FILESYSTEM!\nTODO: ADD BETTER CHECKING FOR FREE SPACE ON LINUX
          (if _returnvalue_5
            (goto _label)
            (else
              (set `local.LocalFinal` 0)))))))
  (return _output_get))

(fn `GetSpecifiedGameMetaPath`
  (params (InName :type Name))
  (returns (ReturnValue :type String))
  (return (`KismetStringLibrary.Concat_StrStr` (`KismetSystemLibrary.GetProjectSavedDirectory`) "meta/" (`KismetStringLibrary.Conv_NameToString` InName) "/")))

(fn `GetUmuPath`
  (returns (Binary :type String) (Directory :type String))
  (bind _returnvalue (`KismetSystemLibrary.GetProjectSavedDirectory`))
  (return (`KismetStringLibrary.Concat_StrStr` _returnvalue "umu/umu-run") (`KismetStringLibrary.Concat_StrStr` _returnvalue "umu/")))

(fn `IsPathSafe?`
  (params (A :type String))
  (returns (ReturnValue :type Boolean))
  (return (not (or (`KismetStringLibrary.Contains` A "C:\\Windows") (`KismetStringLibrary.EqualEqual_StrStr` A "C:\\")))))

(fn `MakeDefaultInstallDir`
  (returns (FinalInstallDir :type String))
  (locals (FinalInstallDirectory :type String))
  (switch `string` (`GameplayStatics.GetPlatformName`)
    (:`Windows`
      (set `local.FinalInstallDirectory` (`KismetStringLibrary.Concat_StrStr` (`KismetSystemLibrary.GetProjectSavedDirectory`) "Games/")))
    (:`Linux`
      (set `local.FinalInstallDirectory` (`KismetTextLibrary.Conv_TextToString` (`|FormatText` "/home/{user}/Games/" (`KismetSystemLibrary.GetPlatformUserName`))))))
  (return (`local.FinalInstallDirectory`)))

(fn `MatchesAnyWildcard`
  (params (FileName :type String) (Wildcards :type "Array of String") (SearchCase :type "ESearchCase Enum" :default "CaseSensitive"))
  (returns (ReturnValue :type Boolean))
  (locals (LocalFound :type Integer))
  (if (`KismetArrayLibrary.Array_IsNotEmpty` Wildcards)
    (for _array_element Wildcards
      (if (`KismetStringLibrary.MatchesWildcard` FileName _array_element SearchCase)
        (`/Engine/EditorBlueprintResources/StandardMacros.IncrementInt` (`local.LocalFound`)))))
  (return (!= (`local.LocalFound`) 0)))

(fn `SetBorderBackgroundColor`
  (params (Target :type "Border Object Reference") (InColor :type "LinearColor Structure"))
  (set `Border.BrushColor` InColor Target))

(fn `SetBorderOutlineSettings`
  (params (Border :type "Border Object Reference") (OutlineSettings :type "SlateBrushOutlineSettings Structure"))
  (bind _background (`Border.Background` Border))
  (bind (_tintcolor _drawas _tiling _mirroring _imagesize _margin _resourceobject) (break `SlateBrush` _background))
  (if (`|EnumEquality` (`.DrawAs` (break `SlateBrush` _background)) "RoundedBox")
    (`Border.SetBrush` Border (make `SlateBrush` _tintcolor _drawas _tiling _mirroring _imagesize _margin _resourceobject OutlineSettings))))

(fn `SetBordersBackgroundColor`
  (params (InColor :type "LinearColor Structure") (Array :type "Array of Border Object Reference"))
  (bind (_r _g _b) (`KismetMathLibrary.BreakColor` InColor))
  (for _array_element Array
    (`/Engine/EditorBlueprintResources/StandardMacros.IsValid` (`.ResourceObject` (break `SlateBrush` (`Border.Background` _array_element)))
      (:`Is Not Valid`
        (set `Border.BrushColor` (`KismetMathLibrary.MakeColor` _r _g _b (`.A` (break `LinearColor` (`Border.BrushColor` _array_element)))) _array_element)))))

(fn `SetButtonStyles`
  (params (InputPin :type "Array of Button Object Reference") (BackgroundColor :type "LinearColor Structure (by ref)"))
  (locals (LocalStyle :type "ButtonStyle Structure"))
  (bind ((`Normal` _normal) (`Hovered` _hovered) (`Pressed` _pressed) (`Disabled` _disabled)) (break `ButtonStyle` (`local.LocalStyle`)))
  (for _array_element InputPin
    (bind _output_get (set `local.LocalStyle` (`Button.WidgetStyle` _array_element)))
    (bind _returnvalue (`ButtonStyleHelper.SetButtonBackgroundColorWithAlpha` _output_get BackgroundColor (`.A` (break `LinearColor` (`.SpecifiedColor` (break `SlateColor` (`.TintColor` (break `SlateBrush` _normal)))))) (`.A` (break `LinearColor` (`.SpecifiedColor` (break `SlateColor` (`.TintColor` (break `SlateBrush` _hovered)))))) (`.A` (break `LinearColor` (`.SpecifiedColor` (break `SlateColor` (`.TintColor` (break `SlateBrush` _pressed)))))) (`.A` (break `LinearColor` (`.SpecifiedColor` (break `SlateColor` (`.TintColor` (break `SlateBrush` _disabled))))))))
    (`Button.SetStyle` _array_element _returnvalue)))

(fn `SetThemmingInParent`
  (params (Parent :type "Border Object Reference (by ref)") (ButtonAccentColor :type "LinearColor Structure (by ref)") (BorderAccentColor :type "LinearColor Structure (by ref)") (BorderOutlineSettings :type "SlateBrushOutlineSettings Structure (by ref)") (ButtonOutlineSettings :type "SlateBrushOutlineSettings Structure (by ref)"))
  (`self.SetBorderOutlineSettings` Parent BorderOutlineSettings)
  (`self.SetBorderBackgroundColor` Parent BorderAccentColor)
  (bind _outwidgets (`WidgetUtilsLibrary.GetAllChildrenOfClassRecursive` Parent "/Script/UMG.Button"))
  (for _array_element _outwidgets
    (bind _asbutton (cast `Button` _array_element))
    (bind _returnvalue (`ButtonStyleHelper.SetButtonBackgroundColorWithAlpha` (`Button.WidgetStyle` _asbutton) ButtonAccentColor))
    (bind _returnvalue_2 (`ButtonStyleHelper.SetButtonOutlineSettings` _returnvalue ButtonOutlineSettings))
    (`Button.SetStyle` _asbutton _returnvalue_2)))

(fn `SetVisibility (bool)`
  (params (Variable :type Boolean) (Widget :type "Widget Object Reference"))
  (if Variable
    (set `Widget.Visibility` "Visible" Widget)
    (else
      (set `Widget.Visibility` "Collapsed" Widget))))

(fn `SetWindowed`
  (bind _returnvalue (`GameUserSettings.GetGameUserSettings`))
  (bind (_x _y) (break `IntPoint` (`GameUserSettings.GetDesktopResolution` _returnvalue)))
  (`GameUserSettings.SetScreenResolution` _returnvalue (make `IntPoint` (/ _x 1.3) (/ _y 1.3)))
  (`GameUserSettings.SetFullscreenMode` _returnvalue "Windowed")
  (`GameUserSettings.ApplySettings` _returnvalue false))

(fn `VerifyFreeDiskSpace`
  (params (Path :type String) (RequiredFreeSpaceInMB :type Integer64))
  (returns (ReturnValue :type Boolean))
  (return (not (< (`self.GetPlatformFreeDiskSpaceInMB` Path) RequiredFreeSpaceInMB))))