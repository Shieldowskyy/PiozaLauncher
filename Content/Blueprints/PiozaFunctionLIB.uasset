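; Blueprint function library of file-name and path helpers for per-game metadata stored under the project's Saved/meta folder.
; CleanFilename chains Replace calls to strip some filename-unsafe characters from a string.
; GetSpecifiedGameMetaPath builds a game's meta folder path from its name.
; GetMetaPath builds the absolute path to a file in that folder and also returns whether that file exists.
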(fn `CleanFilename`
  (params (SourceString :type String))
  (returns (ReturnValue :type String))
  (return (`KismetStringLibrary.Replace` (`KismetStringLibrary.Replace` (`KismetStringLibrary.Replace` (`KismetStringLibrary.Replace` (`KismetStringLibrary.Replace` (`KismetStringLibrary.Replace` SourceString ":") "/") "\\") "?") "<") ">")))

(fn `GetMetaPath`
  (params (GameName :type String) (FileWithExtension :type String))
  (returns (FilePath :type String) (ReturnValue :type Boolean))
  (bind _returnvalue (`KismetSystemLibrary.ConvertToAbsolutePath` (`KismetStringLibrary.Concat_StrStr` (`KismetSystemLibrary.GetProjectSavedDirectory`) "meta/" GameName "/" FileWithExtension)))
  (bind _returnvalue_2 (`FileHelperBPLibrary.IsFile` _returnvalue))
  (return _returnvalue _returnvalue_2))

(fn `GetSpecifiedGameMetaPath`
  (params (InName :type Name))
  (returns (ReturnValue :type String))
  (return (`KismetStringLibrary.Concat_StrStr` (`KismetSystemLibrary.GetProjectSavedDirectory`) "meta/" (`KismetStringLibrary.Conv_NameToString` InName) "/")))