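; ChecksumWorker verifies files in a game directory against MD5 checksums loaded from a file, honoring an ignore list.
; CompareMD5 starts an asynchronous check and relays progress; on completion it merges corrupted and missing files and reports whether all are correct.
; If the checksum file fails to load, nothing is reported.
; The wildcard-based RemoveIgnoredFiles helper is not called here; the ignore list goes straight to the async verifier.
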(event `CompareMD5`
  (params (ChecksumFilePath :type String) (GameDirectoryPath :type String) (FilesToIgnore :type "Array of String"))
  (bind _output_get (set `self.Files to Ignore` FilesToIgnore))
  (bind (_outchecksums _returnvalue) (`ChecksumLibrary.LoadChecksumsFromFile` ChecksumFilePath))
  (if _returnvalue
    (bind _keys (`BlueprintMapLibrary.Map_Keys` _outchecksums))
    (`ChecksumLibraryAsync.VerifyFileListAsync` _keys _outchecksums GameDirectoryPath _output_get "MD5" (delegate `OnProgress`) (delegate `OnComplete`))))

(event `OnProgress`
  (params (ProgressPercent :type "Float (single-precision)") (CurrentFile :type String))
  (`self.OnChecksumProgress` CurrentFile 0 0 false ProgressPercent))

(event `OnComplete`
  (params (Result :type " Structure"))
  (bind _localincorrectfiles (`self.LocalIncorrectFiles`))
  (`KismetArrayLibrary.Array_Append` (`self.LocalIncorrectFiles`) Result_CorruptedFiles)
  (`KismetArrayLibrary.Array_Append` _localincorrectfiles Result_MissingFiles)
  (`self.OnChecksumComplete` (`KismetArrayLibrary.Array_IsEmpty` (`self.LocalIncorrectFiles`)) _localincorrectfiles))

(fn `MatchesAnyWildcard`
  (params (FileName :type String) (Wildcards :type "Array of String") (SearchCase :type "ESearchCase Enum" :default "CaseSensitive"))
  (returns (ReturnValue :type Boolean))
  (locals (LocalFound :type Integer))
  (if (`KismetArrayLibrary.Array_IsNotEmpty` Wildcards)
    (for _array_element Wildcards
      (if (`KismetStringLibrary.MatchesWildcard` FileName _array_element SearchCase)
        (`/Engine/EditorBlueprintResources/StandardMacros.IncrementInt` (`local.LocalFound`)))))
  (return (!= (`local.LocalFound`) 0)))

(fn `RemoveIgnoredFiles`
  (bind _localincorrectfiles (`self.LocalIncorrectFiles`))
  (for _array_element _localincorrectfiles
    (if (`self.MatchesAnyWildcard` _array_element (`self.Files to Ignore`))
      (`KismetArrayLibrary.Array_RemoveItem` _localincorrectfiles _array_element))))