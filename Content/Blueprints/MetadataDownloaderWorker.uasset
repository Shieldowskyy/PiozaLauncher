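; Launcher worker that, on BeginPlay, refreshes cached metadata files and screenshots for every game in the manifest, then signals completion.
; Nested manually advanced loops fetch each game's files sequentially into Saved/meta, updating MainLauncher progress text and bar.
; Remote content size is compared with local file size to skip unchanged files.
; Numbered screenshots download to memory until a failed request or content check ends that game's series, and are saved and texture-cached.
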(event `OnFileDownloadCompleted`
  (params (Result :type "EDownloadToStorageResult Enum" :default "Success") (SavedPath :type String) (Downloader :type "FileToStorageDownloader Object Reference"))
  (switch `EDownloadToStorageResult` Result
    (:`Success`
      (`KismetSystemLibrary.PrintString` (`KismetStringLibrary.Concat_StrStr` "Save file path: " SavedPath) :!label _label)
      (`self.DownloadNextFile`))
    (:`SucceededByPayload`
      (goto _label))
    (:`Cancelled`
      (`/DSHDebugConsole/Blueprints/LIB_DebugConsoleDEFAULT.SendToLog` "NewEnumerator12" (`KismetStringLibrary.Concat_StrStr` "FAILED TO DOWNLOAD FILE FOR PATH:  \n" SavedPath " \neRROR: " (`|GetEnumeratorNameAsString` Result)) :!label _label_2))
    (:`DownloadFailed`
      (goto _label_2))
    (:`SaveFailed`
      (goto _label_2))
    (:`DirectoryCreationFailed`
      (goto _label_2))
    (:`InvalidURL`
      (goto _label_2))
    (:`InvalidSavePath`
      (goto _label_2))))

(event `DownloadNextFile`
  (goto _label_5 :!via `Next`))

(event `NextGame`
  (goto _label_4 :!via `Next`))

(event `DownloadNextScreenshot`
  (bind _output_get (set `self.ScreenshotNumber` (+ (stale _output_get) 1)))
  (`BaseFilesDownloader.GetContentSize` (`KismetStringLibrary.Concat_StrStr` (`self.CurrentMetaGameURL`) "meta/screens/" (`KismetStringLibrary.Concat_StrStr` "screen" (`KismetStringLibrary.Conv_IntToString` (`self.ScreenshotNumber`)) ".jpg")) 1.0 (delegate `ScreenshotContentSize`) :!label _label_3))

(event `OnScreenshotDownloaded`
  (params (DownloadedContent :type "Array of Byte (by ref)") (Result :type "EDownloadToMemoryResult Enum" :default "Success") (Downloader :type "FileToMemoryDownloader Object Reference"))
  (bind _returnvalue (`KismetStringLibrary.Concat_StrStr` (`KismetSystemLibrary.GetProjectSavedDirectory`) "meta/" (`self.CurrentMetaGameName`) "/screens/" (`KismetStringLibrary.Concat_StrStr` "screen" (`KismetStringLibrary.Conv_IntToString` (`self.ScreenshotNumber`)) ".jpg")))
  (bind _returnvalue_2 (`BaseFilesDownloader.BytesToString` DownloadedContent))
  (if (and (`|EnumEquality` Result "Success") (or (`KismetStringLibrary.Contains` _returnvalue_2 "PNG") (not (`KismetStringLibrary.Contains` _returnvalue_2 "DOCTYPE")) (not (`KismetStringLibrary.Contains` _returnvalue_2 "<?xml"))))
    (`KismetSystemLibrary.PrintString` "SAVING PNG FILE..." true true (struct :`R` 0.289773 :`G` 1.0 :`A` 1.0) 5.0)
    (`BaseFilesDownloader.SaveArrayToFile` DownloadedContent _returnvalue)
    (`/Game/Blueprints/Widgets/W_MainLauncher1.CacheTexture2D` (`self.MainLauncher`) _returnvalue)
    (`self.DownloadNextScreenshot`)
    (else
      (`KismetSystemLibrary.PrintString` "NOT A PNG FILE! CANCELLING SAVING PROCESS AND SKIPPING..." false true (struct :`R` 1.0 :`G` 0.104234 :`A` 1.0) 6.0)
      (`self.NextGame`))))

(event `CustomEvent_4`
  (params (BytesReceived :type Integer64) (ContentLength :type Integer64) (ProgressRatio :type "Float (single-precision)")))

(event `ScreenshotContentSize`
  (params (ContentLength :type Integer64))
  (bind _returnvalue (`KismetStringLibrary.Concat_StrStr` "screen" (`KismetStringLibrary.Conv_IntToString` (`self.ScreenshotNumber`)) ".jpg"))
  (bind _returnvalue_2 (`FileNodes.GetFileSize` (`KismetStringLibrary.Concat_StrStr` (`KismetSystemLibrary.GetProjectSavedDirectory`) "meta/" (`self.CurrentMetaGameName`) "/screens/" _returnvalue)))
  (if (== _returnvalue_2 ContentLength)
    (`KismetSystemLibrary.PrintString` "SCREENSHOT IDENTICAL TO CACHED! SKIPPING..." false true (struct :`R` 1.0 :`G` 0.104234 :`A` 1.0) 6.0)
    (`self.DownloadNextScreenshot`)
    (else
      (`FileToMemoryDownloader.DownloadFileToMemory` (`KismetStringLibrary.Concat_StrStr` (`self.CurrentMetaGameURL`) "meta/screens/" _returnvalue) 0.0 "image/x-jpg" false (delegate `CustomEvent_4`) (delegate `OnScreenshotDownloaded`))
      (set `TextBlock.Text` (`|FormatText` "Downloading {filename} for {GameName}..." _returnvalue (`self.CurrentMetaGameName`)) (`/Game/Blueprints/Widgets/W_MainLauncher1.MetadataDesc` (`self.MainLauncher`))))))

(event `MetaContentSize`
  (params (ContentLength :type Integer64))
  (bind _returnvalue (`KismetStringLibrary.Concat_StrStr` (`KismetStringLibrary.Concat_StrStr` (`KismetSystemLibrary.GetProjectSavedDirectory`) "meta/" (`self.CurrentMetaGameName`) "/") (stale `self.ReceiveBeginPlay` _array_element_2)))
  (bind _returnvalue_2 (`FileNodes.GetFileSize` _returnvalue))
  (if (or (== ContentLength _returnvalue_2) (< ContentLength 2048))
    (`KismetSystemLibrary.PrintString` "ASSET IDENTICAL TO CACHED OR TOO SMALL! SKIPPING..." false true (struct :`R` 1.0 :`G` 0.104234 :`A` 1.0) 6.0)
    (`self.DownloadNextFile`)
    (else
      (`FileToStorageDownloader.DownloadFileToStorage` (`KismetStringLibrary.Concat_StrStr` (`self.CurrentMetaGameURL`) "meta/" (stale `self.ReceiveBeginPlay` _array_element_2)) _returnvalue 0.0 "audio/wav" false (delegate `OnFileDownloading`) (delegate `OnFileDownloadCompleted`))
      (bind _result (`|FormatText` "Downloading {filename} for {GameName}..." (stale `self.ReceiveBeginPlay` _array_element_2) (`self.CurrentMetaGameName`)))
      (`KismetSystemLibrary.PrintString` (`KismetTextLibrary.Conv_TextToString` _result) false true (struct :`R` 0.946525 :`G` 1.0 :`A` 1.0) 6.0)
      (set `TextBlock.Text` _result (`/Game/Blueprints/Widgets/W_MainLauncher1.MetadataDesc` (`self.MainLauncher`))))))

(event `OnFileDownloading`
  (params (BytesReceived :type Integer64) (ContentLength :type Integer64) (ProgressRatio :type "Float (single-precision)")))

(event `self.ReceiveBeginPlay`
  (bind ((`minSupportedVersion_43_AF634A1AD4E542208FB2C8470CDB138D` _minsupportedversion) (`latestVersion_45_FB94109C99F44AC28986A983DDE07EDF` _latestversion) (`gamesURLs_37_865694942B944B8390906D59FBAF85BA` _gamesurls)) (break `/Game/Blueprints/Structs/SLauncherManifest` (`self.SLauncher Manifest`)))
  (bind _keys (`BlueprintMapLibrary.Map_Keys` _gamesurls))
  (bind (_array_element _array_index) (`/Game/Blueprints/Libs/PiozaMacroLIB.ForEachLoopWithDelay` _keys :!label _label_4)
    (:`LoopBody`
      (set `self.CurrentMetaGameName` _array_element)
      (set `self.CurrentMetaGameURL` (`BlueprintMapLibrary.Map_Find` _gamesurls (`self.CurrentMetaGameName`)))
      (bind _returnvalue (`KismetArrayLibrary.Array_Length` _keys))
      (set `TextBlock.Text` (`|FormatText` "Refreshing metadata ({current}/{length})" (+ _array_index 1) _returnvalue) (`/Game/Blueprints/Widgets/W_MainLauncher1.MetadataText` (`self.MainLauncher`)))
      (`ProgressBar.SetPercent` (`/Game/Blueprints/Widgets/W_MainLauncher1.RefreshingProgress` (`self.MainLauncher`)) (/ (/ 100 (- _returnvalue _array_index)) 100.0))
      (bind _returnvalue_2 (`BlueprintFileUtilsBPLibrary.MakeDirectory` (`KismetStringLibrary.Concat_StrStr` (`KismetSystemLibrary.GetProjectSavedDirectory`) "meta/" (`self.CurrentMetaGameName`)) true))
      (if _returnvalue_2
        (bind _array_element_2 (`/Game/Blueprints/Libs/PiozaMacroLIB.ForEachLoopWithDelay` (`self.MetaToDownload`) :!label _label_5)
          (:`LoopBody`
            (`BaseFilesDownloader.GetContentSize` (`KismetStringLibrary.Concat_StrStr` (`self.CurrentMetaGameURL`) "meta/" _array_element_2) 1.0 (delegate `MetaContentSize`)))
          (:`Completed`
            (set `self.ScreenshotNumber` 0)
            (goto _label_3)))
        (else
          (`/Game/Blueprints/Widgets/W_MainLauncher1.CustomError` (`self.MainLauncher`) "Failed to create folder tree for games metadata files!\nCheck free disk space or permissions or try reinstalling or updating launcher..."))))
    (:`Completed`
      (`self.OnMetadataDownloadCompleted`))))

(fn `UserConstructionScript`)